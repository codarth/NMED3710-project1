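; BridgeFallingPiece_BP is a bridge piece that breaks away when its trigger box is overlapped.
; The trigger plays a placeholder sound and enables physics on the piece.
; A separate KillBox plays the same sound for any overlap, then prints a debug message if the actor is the FirstPersonCharacter.
; Death and checkpoint respawn logic using TestGameInstance exists but is disconnected, so it never runs.
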(event OnComponentBeginOverlap(TriggerBox)
  (params (OverlappedComponent :type Primitive%20Component%20Object%20Reference) (OtherActor :type Actor%20Object%20Reference) (OtherComp :type Primitive%20Component%20Object%20Reference) (OtherBodyIndex :type Integer) (bFromSweep :type Boolean) (SweepResult :type Hit%20Result%20Structure%20%28by%20ref%29))
  ;[1 1 1] change sounds here, wood breaking
  (Audio|PlaySoundatLocation "/Game/Sound/fire_torch01.fire_torch01" (Transformation|GetWorldLocation (Variables|Default|GetBridgePiece)) "0, 0, 0" 1.0 1.0 0.0 0 0 0)
  (Physics|SetSimulatePhysics (Variables|Default|GetBridgePiece) true))

(event OnComponentBeginOverlap(KillBox)
  (params (OverlappedComponent :type Primitive%20Component%20Object%20Reference) (OtherActor :type Actor%20Object%20Reference) (OtherComp :type Primitive%20Component%20Object%20Reference) (OtherBodyIndex :type Integer) (bFromSweep :type Boolean) (SweepResult :type Hit%20Result%20Structure%20%28by%20ref%29))
  ;[1 1 1] change sounds here, make will helm scream
  (Audio|PlaySoundatLocation "/Game/Sound/fire_torch01.fire_torch01" (Transformation|GetWorldLocation (Variables|Default|GetKillBox)) "0, 0, 0" 1.0 1.0 0.0 0 0 0)
  (bind _asfirst_person_character (Utilities|Casting|CastToFirstPersonCharacter OtherActor))
  (Development|PrintString "deaded"))

(event EventBeginPlay
  (bind _asfirst_person_character (Utilities|Casting|CastToFirstPersonCharacter (Game|GetPlayerCharacter 0)))
  (bind _output_get (Variables|Default|SetplayerRef _asfirst_person_character)))

(fn ConstructionScript)