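; Boulder hazard Blueprint that kills the first-person player on contact.
; When a FirstPersonCharacter overlaps the kill sphere, it prints a death message, disables player 0's input and turns on physics simulation for that character's capsule.
; A one-second delay ends the chain with nothing after it.
; Unconnected leftover nodes hold an alternate overlap check, a sphere physics shutoff and a TwinButtes level load.
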(event OnComponentBeginOverlap(kill_Sphere)
  (params (OverlappedComponent :type Primitive%20Component%20Object%20Reference) (OtherActor :type Actor%20Object%20Reference) (OtherComp :type Primitive%20Component%20Object%20Reference) (OtherBodyIndex :type Integer) (bFromSweep :type Boolean) (SweepResult :type Hit%20Result%20Structure%20%28by%20ref%29))
  (bind _returnvalue (Game|GetPlayerCharacter 0))
  (Utilities|Casting|CastToFirstPersonCharacter OtherActor)
  (Development|PrintString "Kiled by Boulder")
  (Input|DisableInput _returnvalue 0)
  (Physics|SetSimulatePhysics (Variables|/Script/Engine.Character|GetCapsuleComponent _returnvalue) true)
  (Utilities|FlowControl|Delay 1.0))

(event EventBeginPlay)

(event EventTick
  (params (DeltaSeconds :type Float%20%28single-precision%29)))

(event Collision|EventActorBeginOverlap
  (params (OtherActor :type Actor%20Object%20Reference)))

(fn ConstructionScript)