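; finalIdol is a spinning idol actor that is consumed the first time something overlaps its Box trigger.
; Tick rotates the Cube around yaw at RotateSpeed, scaled by delta time.
; The overlap runs once, playing a save-point sound at the box, then after a short delay a male laugh.
; It then destroys the Cube and its PointLight, each behind a validity check.
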(event OnComponentBeginOverlap(Box)
  (params (OverlappedComponent :type Primitive%20Component%20Object%20Reference) (OtherActor :type Actor%20Object%20Reference) (OtherComp :type Primitive%20Component%20Object%20Reference) (OtherBodyIndex :type Integer) (bFromSweep :type Boolean) (SweepResult :type Hit%20Result%20Structure%20%28by%20ref%29))
  (bind _pointlight (Variables|Default|GetPointLight))
  (bind _cube (Variables|Default|GetCube))
  ;[1 1 1] scream sound here
  (Utilities|FlowControl|DoOnce false
    (:Completed
      (Audio|PlaySoundatLocation "/Game/Sound/SavePoint1.SavePoint1" (Transformation|GetWorldLocation (Variables|Default|GetBox)) "0, 0, 0" 1.0 1.0 0.0 0 0 0)
      (Utilities|FlowControl|Delay 1.0)
      ;[1 1 1] scream sound here
      (Audio|PlaySoundatLocation "/Game/Sound/Male_Laugh03.Male_Laugh03" (Transformation|GetWorldLocation (Variables|Default|GetBox)) "0, 0, 0" 1.0 1.0 0.0 0 0 0)
      (Utilities|IsValid _cube
        (:Is%20Valid
          (Components|DestroyComponent _cube)
          (Utilities|IsValid _pointlight
            (:Is%20Valid
              (Components|DestroyComponent _pointlight))))))))

(event EventBeginPlay)

(event Collision|EventActorBeginOverlap
  (params (OtherActor :type Actor%20Object%20Reference)))

(event EventTick
  (params (DeltaSeconds :type Float%20%28single-precision%29))
  (bind _cube (Variables|Default|GetCube))
  (Utilities|IsValid _cube
    (:Is%20Valid
      (Transformation|AddLocalRotation _cube (* (Math|Rotator|MakeRotator 0.0 0.0 (Variables|Default|GetRotateSpeed)) DeltaSeconds) false false))))

(fn ConstructionScript)