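; Shrine checkpoint Blueprint that saves a respawn location when something overlaps its CheckPoint component.
; The overlap plays a save-point sound, then a laugh after a short delay.
; It then writes the Arrow component's world location to the CheckPoint variable on TestGameInstance.
; Finally it destroys the Idol component and its PointLight, leaving the overlap event itself active.
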(event OnComponentBeginOverlap(checkPoint)
  (params (OverlappedComponent :type Primitive%20Component%20Object%20Reference) (OtherActor :type Actor%20Object%20Reference) (OtherComp :type Primitive%20Component%20Object%20Reference) (OtherBodyIndex :type Integer) (bFromSweep :type Boolean) (SweepResult :type Hit%20Result%20Structure%20%28by%20ref%29))
  (bind _idol (Variables|Default|Getidol))
  (bind _pointlight (Variables|Default|GetPointLight))
  ;[1 1 1] change sounds here
  (Audio|PlaySoundatLocation "/Game/Sound/SavePoint1.SavePoint1" (Transformation|GetWorldLocation (Variables|Default|GetcheckPoint)) "0, 0, 0" 1.0 1.0 0.0 0 0 0)
  (Utilities|FlowControl|Delay 0.8)
  ;[1 1 1] change sounds here
  (Audio|PlaySoundatLocation "/Game/Sound/Male_Laugh01.Male_Laugh01" (Transformation|GetWorldLocation (Variables|Default|GetcheckPoint)) "0, 0, 0" 1.0 1.0 0.0 0 0 0)
  (bind _astest_game_instance (Utilities|Casting|CastToTestGameInstance (Game|GetGameInstance)))
  (Variables|/Game/TestGameInstance.TestGameInstance_C|SetcheckPoint _astest_game_instance (Transformation|GetWorldLocation (Variables|Default|GetArrow)))
  (Utilities|IsValid _idol
    (:Is%20Valid
      (Components|DestroyComponent _idol)
      (Utilities|IsValid _pointlight
        (:Is%20Valid
          (Components|DestroyComponent _pointlight))))))

(fn ConstructionScript)