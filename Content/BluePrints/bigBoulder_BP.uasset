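; Rolling boulder trap that kills the first-person player on contact.
; Overlapping the boulder trigger plays a placeholder sound and enables physics on the sphere to set it rolling.
; Kill sphere overlap disables input and flags the player dead, then after a short delay teleports them to the game instance's checkpoint and restores input.
; The boulder itself is never reset.
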(event OnComponentBeginOverlap(kill_Sphere)
  (params (OverlappedComponent :type Primitive%20Component%20Object%20Reference) (OtherActor :type Actor%20Object%20Reference) (OtherComp :type Primitive%20Component%20Object%20Reference) (OtherBodyIndex :type Integer) (bFromSweep :type Boolean) (SweepResult :type Hit%20Result%20Structure%20%28by%20ref%29))
  ;[1 1 1] change sounds here, make a scream
  (Audio|PlaySoundatLocation "/Game/Sound/fire_torch01.fire_torch01" (Transformation|GetWorldLocation (Variables|Default|Getkill_Sphere)) "0, 0, 0" 1.0 1.0 0.0 0 0 0)
  (bind _asfirst_person_character (Utilities|Casting|CastToFirstPersonCharacter OtherActor))
  (Development|PrintString "deaded")
  (Input|DisableInput (stale EventBeginPlay _output_get) 0)
  (Default|SetDeath (stale EventBeginPlay _output_get) true)
  (Utilities|FlowControl|Delay 1.0)
  (bind _astest_game_instance (Utilities|Casting|CastToTestGameInstance (Game|GetGameInstance)))
  (Transformation|Teleport _asfirst_person_character (Variables|/Game/TestGameInstance.TestGameInstance_C|GetcheckPoint _astest_game_instance) "0, 0, 0")
  (Input|EnableInput (stale EventBeginPlay _output_get) 0)
  (Physics|SetSimulatePhysics (Variables|/Script/Engine.Character|GetCapsuleComponent (stale EventBeginPlay _output_get)) false))

(event OnComponentBeginOverlap(boulder_Trigger)
  (params (OverlappedComponent :type Primitive%20Component%20Object%20Reference) (OtherActor :type Actor%20Object%20Reference) (OtherComp :type Primitive%20Component%20Object%20Reference) (OtherBodyIndex :type Integer) (bFromSweep :type Boolean) (SweepResult :type Hit%20Result%20Structure%20%28by%20ref%29))
  ;[1 1 1] boulder rolling
  (Audio|PlaySoundatLocation "/Game/Sound/fire_torch01.fire_torch01" (Transformation|GetWorldLocation (Variables|Default|Getkill_Sphere)) "0, 0, 0" 1.0 1.0 0.0 0 0 0)
  (Physics|SetSimulatePhysics (Variables|Default|GetSphere) true))

(event EventBeginPlay
  (bind _asfirst_person_character (Utilities|Casting|CastToFirstPersonCharacter (Game|GetPlayerCharacter 0)))
  (bind _output_get (Variables|Default|SetplayerRef _asfirst_person_character)))

(event EventTick
  (params (DeltaSeconds :type Float%20%28single-precision%29)))

(event Collision|EventActorBeginOverlap
  (params (OtherActor :type Actor%20Object%20Reference)))

(fn ConstructionScript)