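; Spike trap Blueprint with a moving platform and a kill box that sends the player back to a checkpoint.
; Player overlap starts, after a short delay, a timeline lerping the platform toward EndPoint; leaving stops it after a delay, without reversing.
; Kill box overlaps play placeholder sounds for any actor.
; For the player, they also disable input, set death, wait, teleport to the GameInstance checkpoint and restore input.
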(event OnComponentBeginOverlap(player_Touch)
  (params (OverlappedComponent :type Primitive%20Component%20Object%20Reference) (OtherActor :type Actor%20Object%20Reference) (OtherComp :type Primitive%20Component%20Object%20Reference) (OtherBodyIndex :type Integer) (bFromSweep :type Boolean) (SweepResult :type Hit%20Result%20Structure%20%28by%20ref%29))
  (Utilities|Casting|CastToFirstPersonCharacter OtherActor)
  (Utilities|FlowControl|Delay 0.2)
  (bind _newtrack_0 (Timeline|platform_move Play)
    (:Update
      (Transformation|SetWorldLocation (Variables|Default|GetPlatform) (Math|Vector|Lerp(Vector) (Variables|Default|GetNewVar_0) (Variables|Default|Getend_Loc) _newtrack_0) false false))))

(event OnComponentEndOverlap(player_Touch)
  (params (OverlappedComponent :type Primitive%20Component%20Object%20Reference) (OtherActor :type Actor%20Object%20Reference) (OtherComp :type Primitive%20Component%20Object%20Reference) (OtherBodyIndex :type Integer))
  (Utilities|Casting|CastToFirstPersonCharacter OtherActor)
  (Utilities|FlowControl|Delay 0.5)
  (bind _newtrack_0 (Timeline|platform_move Stop)
    (:Update
      (Transformation|SetWorldLocation (Variables|Default|GetPlatform) (Math|Vector|Lerp(Vector) (Variables|Default|GetNewVar_0) (Variables|Default|Getend_Loc) _newtrack_0) false false))))

(event OnComponentBeginOverlap(kill_box)
  (params (OverlappedComponent :type Primitive%20Component%20Object%20Reference) (OtherActor :type Actor%20Object%20Reference) (OtherComp :type Primitive%20Component%20Object%20Reference) (OtherBodyIndex :type Integer) (bFromSweep :type Boolean) (SweepResult :type Hit%20Result%20Structure%20%28by%20ref%29))
  (bind _playerref (Variables|Default|GetplayerRef))
  ;[1 1 1] stab sound here
  (Audio|PlaySoundatLocation "/Game/Sound/fire_torch01.fire_torch01" (Transformation|GetWorldLocation (Variables|Default|Getkill_box)) "0, 0, 0" 1.0 1.0 0.0 0 0 0)
  ;[1 1 1] scream sound here
  (Audio|PlaySoundatLocation "/Game/Sound/fire_torch01.fire_torch01" (Transformation|GetWorldLocation (Variables|Default|Getkill_box)) "0, 0, 0" 1.0 1.0 0.0 0 0 0)
  (bind _asfirst_person_character (Utilities|Casting|CastToFirstPersonCharacter OtherActor))
  (Development|PrintString "deaded")
  (Input|DisableInput _playerref 0)
  (Default|SetDeath _playerref true)
  (Utilities|FlowControl|Delay 2.0)
  (bind _astest_game_instance (Utilities|Casting|CastToTestGameInstance (Game|GetGameInstance)))
  (bind _returnvalue (Transformation|Teleport _asfirst_person_character (Variables|/Game/TestGameInstance.TestGameInstance_C|GetcheckPoint _astest_game_instance) "0, 0, 0"))
  ;[1 1 1] not needed, for tested
  (Development|PrintString "didnt work" _returnvalue)
  (Input|EnableInput _playerref 0)
  (Physics|SetSimulatePhysics (Variables|/Script/Engine.Character|GetCapsuleComponent _playerref) false))

(event EventBeginPlay
  (Variables|Default|SetNewVar_0 (Transformation|GetWorldLocation (Variables|Default|GetPlatform)))
  (Variables|Default|Setend_Loc (Transformation|GetWorldLocation (Variables|Default|Getend_Point)))
  (Variables|Default|Setkill_loc (Transformation|GetWorldLocation (Variables|Default|Getkill_box)))
  (Components|Timeline|SetPlayRate (Variables|Default|Getplatform_move) (Variables|Default|Getplay_Rate))
  (bind _asfirst_person_character (Utilities|Casting|CastToFirstPersonCharacter (Game|GetPlayerCharacter 0)))
  (Variables|Default|SetplayerRef _asfirst_person_character))

(fn ConstructionScript)