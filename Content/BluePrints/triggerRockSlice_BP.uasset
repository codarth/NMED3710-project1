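; Trigger actor that starts a rockslide from boulder_BP actors tagged RockSlide1 when something overlaps it.
; Each overlap plays a sound at every tagged boulder before checking that the overlapping actor is the FirstPersonCharacter.
; For the player, a nested tag search enables physics on the boulders' spheres, then a delay leads to destroying all tagged actors.
; Class-based search variants remain unconnected.
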(event EventBeginPlay)

(event Collision|EventActorBeginOverlap
  (params (OtherActor :type Actor%20Object%20Reference))
  (bind _outactors (Actor|GetAllActorswithTag "RockSlide1"))
  (for _array_element _outactors
    (bind _asboulder_bp (Utilities|Casting|CastToboulder_BP _array_element))
    ;[1 1 1] roackslide sounds
    (Audio|PlaySoundatLocation "/Game/Sound/fire_torch01.fire_torch01" (Transformation|GetWorldLocation (Variables|/Script/Engine.Actor|GetRootComponent _asboulder_bp)) "0, 0, 0" 1.0 1.0 0.0 0 0 0)
    (Utilities|Casting|CastToFirstPersonCharacter OtherActor)
    (bind _outactors_2 (Actor|GetAllActorswithTag "RockSlide1"))
    (for _array_element_2 _outactors_2
      (bind _asboulder_bp_2 (Utilities|Casting|CastToboulder_BP _array_element_2))
      (Physics|SetSimulatePhysics (Variables|/Game/BluePrints/boulder_BP.boulder_BP_C|GetSphere _asboulder_bp_2) true)
      (Utilities|FlowControl|Delay 15.0)
      (bind _outactors_3 (Actor|GetAllActorswithTag "RockSlide1"))
      (for _array_element_3 _outactors_3
        (Actor|DestroyActor _array_element_3)))))

(event EventTick
  (params (DeltaSeconds :type Float%20%28single-precision%29)))

(fn ConstructionScript)