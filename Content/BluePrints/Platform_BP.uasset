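; Moving platform that travels to an end point when the first-person player enters its touch trigger and returns when they leave.
; BeginPlay caches the platform's start and EndPoint world locations and applies a configurable PlayRate.
; Overlap begin and end play or reverse a timeline after a half-second delay.
; The timeline lerps the platform between both locations without sweeping.
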(event OnComponentBeginOverlap(player_Touch)
  (params (OverlappedComponent :type Primitive%20Component%20Object%20Reference) (OtherActor :type Actor%20Object%20Reference) (OtherComp :type Primitive%20Component%20Object%20Reference) (OtherBodyIndex :type Integer) (bFromSweep :type Boolean) (SweepResult :type Hit%20Result%20Structure%20%28by%20ref%29))
  (Utilities|Casting|CastToFirstPersonCharacter OtherActor)
  (Utilities|FlowControl|Delay 0.5)
  (bind _newtrack_0 (Timeline|platform_move Play)
    (:Update
      (Transformation|SetWorldLocation (Variables|Default|GetPlatform) (Math|Vector|Lerp(Vector) (Variables|Default|GetNewVar_0) (Variables|Default|Getend_Loc) _newtrack_0) false false))))

(event OnComponentEndOverlap(player_Touch)
  (params (OverlappedComponent :type Primitive%20Component%20Object%20Reference) (OtherActor :type Actor%20Object%20Reference) (OtherComp :type Primitive%20Component%20Object%20Reference) (OtherBodyIndex :type Integer))
  (Utilities|Casting|CastToFirstPersonCharacter OtherActor)
  (Utilities|FlowControl|Delay 0.5)
  (bind _newtrack_0 (Timeline|platform_move Reverse)
    (:Update
      (Transformation|SetWorldLocation (Variables|Default|GetPlatform) (Math|Vector|Lerp(Vector) (Variables|Default|GetNewVar_0) (Variables|Default|Getend_Loc) _newtrack_0) false false))))

(event EventBeginPlay
  (Variables|Default|SetNewVar_0 (Transformation|GetWorldLocation (Variables|Default|GetPlatform)))
  (Variables|Default|Setend_Loc (Transformation|GetWorldLocation (Variables|Default|Getend_Point)))
  (Components|Timeline|SetPlayRate (Variables|Default|Getplatform_move) (Variables|Default|Getplay_Rate)))

(fn ConstructionScript)