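; Trigger volume that sets off a rockslide of boulder_BP actors tagged "RockSlide2".
; On box overlap it plays a debris sound at each tagged boulder, before the FirstPersonCharacter check, so any overlapping actor triggers the audio.
; For the player, nested tag lookups enable physics on the boulders, then destroy all tagged actors after a delay.
; Older class-based lookup nodes remain unconnected.
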(event OnComponentBeginOverlap(Box)
  (params (OverlappedComponent :type Primitive%20Component%20Object%20Reference) (OtherActor :type Actor%20Object%20Reference) (OtherComp :type Primitive%20Component%20Object%20Reference) (OtherBodyIndex :type Integer) (bFromSweep :type Boolean) (SweepResult :type Hit%20Result%20Structure%20%28by%20ref%29))
  (bind _outactors (Actor|GetAllActorswithTag "RockSlide2"))
  (for _array_element _outactors
    (bind _asboulder_bp (Utilities|Casting|CastToboulder_BP _array_element))
    ;[1 1 1] roackslide sounds
    (Audio|PlaySoundatLocation "/Game/Sound/Rock_DebrisFall02.Rock_DebrisFall02" (Transformation|GetWorldLocation (Variables|/Script/Engine.Actor|GetRootComponent _asboulder_bp)) "0, 0, 0" 1.0 1.0 0.0 0 0 0)
    (Utilities|Casting|CastToFirstPersonCharacter OtherActor)
    (bind _outactors_2 (Actor|GetAllActorswithTag "RockSlide2"))
    (for _array_element_2 _outactors_2
      (bind _asboulder_bp_2 (Utilities|Casting|CastToboulder_BP _array_element_2))
      (Physics|SetSimulatePhysics (Variables|/Game/BluePrints/boulder_BP.boulder_BP_C|GetSphere _asboulder_bp_2) true)
      (Utilities|FlowControl|Delay 1e+01)
      (bind _outactors_3 (Actor|GetAllActorswithTag "RockSlide2"))
      (for _array_element_3 _outactors_3
        (Actor|DestroyActor _array_element_3)))))

(event EventBeginPlay)

(event EventTick
  (params (DeltaSeconds :type Float%20%28single-precision%29)))

(fn ConstructionScript)